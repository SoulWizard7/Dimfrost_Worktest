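; Base runner character that reacts to line of sight with the player and can be eliminated by projectiles.
; Ninja types periodically line-trace to the player, switching from Active to MoveToPole when sight is lost and back when regained.
; Projectile hits stop behaviour and ragdoll the mesh with an impulse away from the projectile.
; ResetRagdoll reattaches the mesh at its cached transform and clears elimination.
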(event OnComponentHit(CapsuleComponent)
  (params (HitComponent :type Primitive%20Component%20Object%20Reference) (OtherActor :type Actor%20Object%20Reference) (OtherComp :type Primitive%20Component%20Object%20Reference) (NormalImpulse :type Vector :default "0, 0, 0") (Hit :type Hit%20Result%20Structure%20%28by%20ref%29))
  (bind _mesh (Variables|Character|GetMesh))
  (Utilities|Casting|CastToBP_FirstPersonProjectile OtherActor)
  (Class|DWRunnerCharacter|StopBehaviour)
  ;[1 0.2044 0.1546] Ragdoll
  (Collision|SetCollisionEnabled (Variables|Default|GetCapsuleComponent) "NoCollision")
  (Collision|SetCollisionEnabled _mesh "PhysicsOnly")
  (Physics|SetSimulatePhysics _mesh true)
  (Physics|AddImpulse _mesh (* (Math|Vector|Normalize (- (Transformation|GetActorLocation) (Transformation|GetActorLocation OtherActor))) 2e+04) "None" false)
  (Variables|Default|SetbIsEliminated true))

(event EventBeginPlay
  ;[0.5289 1 0.7245] BEGINPLAY
  (Variables|Default|SetDefaultTransform (Transformation|GetRelativeTransform (Variables|Character|GetMesh)))
  (Utilities|FlowControl|Delay 1.0)
  (Variables|Default|SetPlayerActor (Game|Player|GetPlayerPawn 0))
  (switch Utilities|FlowControl|Switch|SwitchonERunnerType (Variables|Default|GetCurrentType)
    (:Ninja
      (Variables|Default|SetTimer (Variables|Default|GetTimeBetweenLOSCheck)))))

(event EventResetRagdoll
  (bind _mesh (Variables|Character|GetMesh))
  ;[1 0.2044 0.1546] Ragdoll
  (Physics|SetSimulatePhysics _mesh false)
  (Collision|SetCollisionEnabled (Variables|Default|GetCapsuleComponent) "QueryAndPhysics")
  (Collision|SetCollisionEnabled _mesh "QueryOnly")
  (Transformation|AttachComponentToComponent _mesh (Variables|Default|GetCapsuleComponent) "None" "KeepRelative" "KeepRelative" "KeepRelative" true)
  (Transformation|SetRelativeTransform (Variables|Character|GetMesh) (Variables|Default|GetDefaultTransform) false false)
  (Variables|Default|SetbIsEliminated false))

(event EventTick
  (params (DeltaSeconds :type Float%20%28single-precision%29))
  (switch Utilities|FlowControl|Switch|SwitchonERunnerType (Variables|Default|GetCurrentType)
    (:Ninja
      ;[1 0.5395 0.9413] Perception
      (bind _output_get (Variables|Default|SetTimer (- (Variables|Default|GetTimer) DeltaSeconds)))
      (if (< _output_get 0.0)
        (CallFunction|CheckLOS)
        (Variables|Default|SetTimer (Variables|Default|GetTimeBetweenLOSCheck))))))

(fn ConstructionScript)

(fn CheckLOS
  (if (!= (Variables|Default|GetPlayerActor) 0)
    (bind _outhit (Collision|LineTraceByChannel (Transformation|GetActorLocation) (Transformation|GetActorLocation (Variables|Default|GetPlayerActor)) "TraceTypeQuery1" false 0 "None"))
    (Variables|Default|SetHasLOS (== (Variables|Default|GetPlayerActor) (.HitActor (Collision|BreakHitResult _outhit))))
    (if (and (Utilities|Enum|Equal(Enum) (Variables|Default|GetCurrentState) "Active") (not (Variables|Default|GetHasLOS)))
      (Class|DWRunnerCharacter|ChangeRunnerState "MoveToPole")
      (elif (and (Variables|Default|GetHasLOS) (Utilities|Enum|Equal(Enum) (Variables|Default|GetCurrentState) "MoveToPole"))
        (Class|DWRunnerCharacter|ChangeRunnerState "Active")))))
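; BP_PoleGameManager runs the round flow for a runner game, from start countdown to winner screen and restart.
; BeginPlay creates the start and end widgets, and Tick starts the game once the start widget's timer runs out.
; During play, a non-eliminated runner overlapping the Capsule, or a PlayerWinsRound call, shows the end screen with the winner unless already displayed.
; RestartGame clears widgets, resets the countdown and marks the game unstarted.
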(event OnComponentBeginOverlap(Capsule)
  (params (OverlappedComponent :type Primitive%20Component%20Object%20Reference) (OtherActor :type Actor%20Object%20Reference) (OtherComp :type Primitive%20Component%20Object%20Reference) (OtherBodyIndex :type Integer) (bFromSweep :type Boolean) (SweepResult :type Hit%20Result%20Structure%20%28by%20ref%29))
  (bind _wb_endgame (Variables|Default|GetWB_EndGame))
  ;[0.6663 0.6413 1] GAME OVER UI ACTIVATION
  (if (not (UserInterface|Viewport|IsinViewport (Variables|Default|GetWB_EndGame)))
    (if (Variables|Default|GetbGameHasStarted)
      (bind _asbp_runner_base (Utilities|Casting|CastToBP_RunnerBase OtherActor))
      (if (not (Variables|/Script/Dimfrost_Worktest.DW_RunnerCharacter|GetbIsEliminated _asbp_runner_base))
        (Variables|/Game/BluePrints/WB_EndGame.WB_EndGame_C|SetWinner _wb_endgame (Utilities|String|EnumtoString (Variables|/Script/Dimfrost_Worktest.DW_RunnerCharacter|GetCurrentType _asbp_runner_base)))
        (UserInterface|Viewport|AddtoViewport _wb_endgame 0)))))

(event Custom|RestartGame
  (bind _wb_start (Variables|Default|GetWB_Start))
  ;[0.5501 1 0.6837] RESTART GAME
  (Viewport|RemoveAllWidgets)
  (Variables|/Game/BluePrints/WB_Start.WB_Start_C|SetStartTimer _wb_start 5.0)
  (UserInterface|Viewport|AddtoViewport _wb_start 0)
  (Variables|Default|SetbGameHasStarted false))

(event EventBeginPlay
  ;[1 0.9663 0.4973] INIT UI AT BEGIN PLAY
  (bind _returnvalue (UserInterface|CreateWidget (Variables|Default|GetWidget_EndGame)))
  (Variables|Default|SetWB_EndGame _returnvalue)
  (bind _returnvalue_2 (UserInterface|CreateWidget (Variables|Default|GetWidget_StartGame)))
  (bind _output_get (Variables|Default|SetWB_Start _returnvalue_2))
  (UserInterface|Viewport|AddtoViewport _output_get 0)
  (Variables|/Game/BluePrints/WB_Start.WB_Start_C|SetStartTimer _output_get 5.0))

(event EventPlayerWinsRound
  (bind _wb_endgame (Variables|Default|GetWB_EndGame))
  ;[0.6663 0.6413 1] GAME OVER UI ACTIVATION
  (if (not (UserInterface|Viewport|IsinViewport (Variables|Default|GetWB_EndGame)))
    (Variables|/Game/BluePrints/WB_EndGame.WB_EndGame_C|SetWinner _wb_endgame "Player")
    (UserInterface|Viewport|AddtoViewport _wb_endgame 0)))

(event EventTick
  (params (DeltaSeconds :type Float%20%28single-precision%29))
  ;[1 0.5654 0.8843] START GAME TIMER
  (if (not (Variables|Default|GetbGameHasStarted))
    (if (not (> (Variables|/Game/BluePrints/WB_Start.WB_Start_C|GetStartTimer (Variables|Default|GetWB_Start)) 0.0))
      (Class|DWGameManager|StartGame)
      (Viewport|RemoveAllWidgets))))

(fn ConstructionScript)